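; Manages the in-game piano-style keyboard and the per-room musical ritual puzzle played on it, plus randomly timed background music.
; MIDI or other note calls spawn soundset sounds from data tables, driving key highlights and notebar visuals; released notes fade on Tick.
; While playing, a metronome and four-segment song timer check recent or held notes against the active room's keynotes.
; Misses rewind the segment; completion finishes the room, potentially switching lighting or ending the game.
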(event `self.ReceiveBeginPlay`
  (bind _returnvalue (`GameplayStatics.GetActorOfClass` "/Game/Game/NoteBarRendering/BP_NotebarRenderer.BP_NotebarRenderer_C"))
  (set `self.NotebarRendererRef` _returnvalue)
  (`self.GetRoomRefs`)
  (`self.RandomIntervalUntilMusic`))

(event `RandomIntervalUntilMusic`
  (`KismetSystemLibrary.Delay` (`KismetMathLibrary.RandomFloatInRange` 30.0 60.0))
  (if (`self.KeyboardIsShown`)
    (`self.RandomIntervalUntilMusic`)
    (else
      (bind _returnvalue (`GameplayStatics.CreateSound2D` (`KismetArrayLibrary.Array_Random` (`|MakeArray` "/Game/Sound/Music/2025_18_06_Jeanne__GAMES_Room_A__DRAFT1__1_.2025_18_06_Jeanne__GAMES_Room_A__DRAFT1__1_" "/Game/Sound/Music/2025_18_06_Jeanne__GAMES_Room_b__DRAFT1_2__1_.2025_18_06_Jeanne__GAMES_Room_b__DRAFT1_2__1_" :!type "SoundBase Object Reference")) 1.0 1.0 0.0 null false false))
      (bind _output_get (set `self.MusicRef` _returnvalue))
      (`AudioComponent.Play` _output_get 0.0))))

(event `FadeoutMusic`
  (bind _musicref (`self.MusicRef`))
  (bind _musicref_2 (`self.MusicRef`))
  (`/Engine/EditorBlueprintResources/StandardMacros.IsValid` _musicref_2
    (:`Is Valid`
      (if (`AudioComponent.IsPlaying` _musicref_2)
        (bind (_direction _volume) (`Timeline|Timeline` :!via `PlayFromStart`)
          (:`Update`
            (if (== _volume 0.0)
              (`AudioComponent.Stop` _musicref)
              (`ActorComponent.K2_DestroyComponent` _musicref)
              (else
                (`AudioComponent.SetVolumeMultiplier` (`self.MusicRef`) _volume))))
          (:`Finished`
            (`self.RandomIntervalUntilMusic`)))))))

(event `Initialize`
  (bind _midicontroller (`self.MidiController`))
  (bind _deviceid (`MIDIDeviceManager.GetDefaultMIDIInputDeviceID`))
  (bind _returnvalue (`MIDIDeviceManager.CreateMIDIDeviceInputController` _deviceid))
  (`/Engine/EditorBlueprintResources/StandardMacros.IsValid` _returnvalue
    (:`Is Valid`
      (set `self.MidiController` _returnvalue)
      (add `MIDIDeviceInputController.OnMIDINoteOn` _midicontroller (delegate `OnMidiNoteOn_Event`))
      (add `MIDIDeviceInputController.OnMIDINoteOff` _midicontroller (delegate `OnMidiNoteOff_Event`)))
    (:`Is Not Valid`
      _))
  (bind _asbp_fp_character (cast `/Game/Player/Blueprints/BP_FP_Character` (`GameplayStatics.GetPlayerPawn` 0)))
  (bind _output_get (set `self.PlayerRef` _asbp_fp_character))
  (bind _ui_ref (`/Game/Player/Blueprints/BP_FP_Character.UI_Ref` _output_get))
  (add `/Game/Widgets/W_IngameMainUI.OnKeyboardShown` _ui_ref (delegate `ToggleStarted`))
  (add `/Game/Widgets/W_IngameMainUI.OnKeyboardHidden` _ui_ref (delegate `ToggleFinished`)))

(event `ToggleStarted`
  (set `self.KeyboardIsShown` true))

(event `ToggleFinished`
  (set `self.KeyboardIsShown` false))

(event `OnMidiNoteOn_Event`
  (params (MIDIDeviceController :type "MIDIDeviceInputController Object Reference") (Timestamp :type Integer) (Channel :type Integer) (Note :type Integer) (Velocity :type Integer))
  (`self.StartPlayingNote` Note Velocity true))

(event `OnMidiNoteOff_Event`
  (params (MIDIDeviceController :type "MIDIDeviceInputController Object Reference") (Timestamp :type Integer) (Channel :type Integer) (Note :type Integer) (Velocity :type Integer))
  (`self.StopPlayingNote` Note true))

(event `self.ReceiveTick`
  (params (DeltaSeconds :type "Float (single-precision)"))
  (if (`self.KeyboardIsShown`)
    (if (`self.IsPlaying`)
      (`self.MetronomeTimer`)
      (`self.ProgressSong`))
    (else
      (set `self.IsPlaying` false)))
  (for _array_element (`self.FadingNotes`)
    (bind (_note _octave _soundset _soundwave _spawnedorder _starttime _heldtime _audioref) (break `/Game/Game/Utilities/S_NoteInfo` _array_element))
    (`/Engine/EditorBlueprintResources/StandardMacros.IsValid` _audioref
      (:`Is Valid`
        (bind _returnvalue (`KismetMathLibrary.FInterpTo` (`AudioComponent.VolumeMultiplier` _audioref) 0.0 DeltaSeconds 8.0))
        (`AudioComponent.SetVolumeMultiplier` _audioref _returnvalue)
        (if (<= _returnvalue 0.0)
          (clear `AudioComponent.OnAudioPlaybackPercent` _audioref)
          (`/Game/Game/NoteBarRendering/BP_NotebarRenderer.StopSoundbar` (`self.NotebarRendererRef`) _array_element :!label _label)
          (`KismetArrayLibrary.Array_RemoveItem` (`self.FadingNotes`) _array_element)))
      (:`Is Not Valid`
        (goto _label)))))

(fn `AddAttemptedNote`
  (params (Note :type "Integer (by ref)"))
  (`KismetArrayLibrary.Array_Add` (`self.CurrentAttemptedKeynotes`) Note)
  (bind _asbp_fp_character (cast `/Game/Player/Blueprints/BP_FP_Character` (`GameplayStatics.GetPlayerPawn` 0)))
  (`/Game/Widgets/W_KeyboardInterface.InvalidateKeyNote` (`/Game/Widgets/W_IngameMainUI.W_KeyboardInterface` (`/Game/Player/Blueprints/BP_FP_Character.UI_Ref` _asbp_fp_character)) Note false true))

(fn `AddUsedNote`
  (params (Note :type "Integer (by ref)"))
  (bind _asbp_fp_character (cast `/Game/Player/Blueprints/BP_FP_Character` (`GameplayStatics.GetPlayerPawn` 0)))
  (`/Game/Widgets/W_KeyboardInterface.InvalidateKeyNote` (`/Game/Widgets/W_IngameMainUI.W_KeyboardInterface` (`/Game/Player/Blueprints/BP_FP_Character.UI_Ref` _asbp_fp_character)) Note false false)
  (`KismetArrayLibrary.Array_Add` (`self.CurrentUsedKeynotes`) Note))

(fn `FailedSegment`
  (bind _returnvalue (- (`self.SongProgression`) 1))
  (set `self.SongProgression` _returnvalue)
  (bind _output_get (set `self.SongTime` (+ (* (/ (`self.TotalPlayLength`) 4.0) _returnvalue) 0.1)))
  (`/Game/Widgets/W_SongTimer.UpdateCursorPosition` (`/Game/Widgets/W_IngameMainUI.W_SongTimer` (`/Game/Player/Blueprints/BP_FP_Character.UI_Ref` (`self.PlayerRef`))) (/ _output_get (`self.TotalPlayLength`)))
  (set `self.CurrentCheckForKeynoteTimer` 0.0)
  (`BlueprintMapLibrary.Map_Clear` (`self.NoteHistory`)))

(fn `GetRoomRefs`
  (bind _outactors (`GameplayStatics.GetAllActorsOfClass` "/Game/Game/BP_RoomDivider.BP_RoomDivider_C"))
  (for _array_element _outactors
    (`BlueprintMapLibrary.Map_Add` (`self.RoomRefs`) (`/Game/Game/BP_RoomDivider.ForwardRoom` _array_element) _array_element)))

(fn `MetronomeTimer`
  (locals (ShouldTock :type Boolean) (TimeBetweenTicks :type "Float (double-precision)"))
  (set `local.TimeBetweenTicks` (/ 60.0 (`KismetMathLibrary.Conv_IntToDouble` (`self.BPM`))))
  (bind _output_get (set `self.TimeSinceLastSound` (+ (`self.TimeSinceLastSound`) (`GameplayStatics.GetWorldDeltaSeconds`))))
  (if (> _output_get (`local.TimeBetweenTicks`))
    (set `self.TimeSinceLastSound` (- (`self.TimeSinceLastSound`) (`local.TimeBetweenTicks`)))
    (if (`self.KeyboardIsShown`)
      (if (`local.ShouldTock`)
        (`GameplayStatics.PlaySound2D` "/Game/Sound/GeneralSFX/MidiInteraction/Tock.Tock" 1.0 1.0 0.0 null null)
        (else
          (`GameplayStatics.PlaySound2D` "/Game/Sound/GeneralSFX/MidiInteraction/Tick.Tick" 1.0 1.0 0.0 null null)))
      (set `local.ShouldTock` (not (`local.ShouldTock`))))))

(fn `NoteOctaveToNote`
  (params (Note :type "/Game/Game/Utilities/E_Notes Enum" :default "NewEnumerator0") (Octave :type Integer))
  (returns (NoteOut :type Integer))
  (return (select `int` Octave :`0` 0 :`1` 0 :`2` (select `/Game/Game/Utilities/E_Notes` Note :`NewEnumerator0` 48 :`NewEnumerator1` 49 :`NewEnumerator2` 50 :`NewEnumerator3` 51 :`NewEnumerator4` 52 :`NewEnumerator5` 53 :`NewEnumerator6` 54 :`NewEnumerator7` 55 :`NewEnumerator8` 56 :`NewEnumerator9` 57 :`NewEnumerator13` 58 :`NewEnumerator10` 59) :`3` (select `/Game/Game/Utilities/E_Notes` Note :`NewEnumerator0` 60 :`NewEnumerator1` 61 :`NewEnumerator2` 62 :`NewEnumerator3` 63 :`NewEnumerator4` 64 :`NewEnumerator5` 65 :`NewEnumerator6` 66 :`NewEnumerator7` 67 :`NewEnumerator8` 68 :`NewEnumerator9` 69 :`NewEnumerator13` 70 :`NewEnumerator10` 71) :`4` 72)))

(fn `NoteToNoteOctave`
  (params (NoteIn :type Integer))
  (returns (NoteOut :type "/Game/Game/Utilities/E_Notes Enum") (Octave :type Integer))
  (return (select `int` (mod NoteIn 12) :`0` "NewEnumerator0" :`1` "NewEnumerator1" :`2` "NewEnumerator2" :`3` "NewEnumerator3" :`4` "NewEnumerator4" :`5` "NewEnumerator5" :`6` "NewEnumerator6" :`7` "NewEnumerator7" :`8` "NewEnumerator8" :`9` "NewEnumerator9" :`10` "NewEnumerator13" :`11` "NewEnumerator10" :!type "/Game/Game/Utilities/E_Notes Enum") (/ (+ NoteIn 47) 12)))

(fn `ProgressSong`
  (locals (IndexToCheck :type Integer) (IsPlayingKeynote :type Boolean))
  (bind _notehistory (`self.NoteHistory`))
  (bind _playerref (`self.PlayerRef`))
  (bind _returnvalue (`BlueprintMapLibrary.Map_Length` _notehistory))
  (bind _returnvalue_2 (- (`local.IndexToCheck`) 1))
  (bind _activeroom (`/Game/Player/Blueprints/BP_FP_Character.ActiveRoom` _playerref))
  (bind (_note _octave _soundset _soundwave _spawnedorder _starttime _heldtime) (break `/Game/Game/Utilities/S_NoteInfo` (`BlueprintMapLibrary.Map_Find` _notehistory (`local.IndexToCheck`))))
  (bind _noteout (`self.NoteOctaveToNote` _note _octave))
  (bind _keynotes (`/Game/Game/BP_RoomDivider.Keynotes` (`BlueprintMapLibrary.Map_Find` (`self.RoomRefs`) (`/Game/Player/Blueprints/BP_FP_Character.ActiveRoom` (`self.PlayerRef`)))))
  (bind _output (`|GetArrayItem` (`/Game/Game/BP_RoomDivider.Keynotes` (`BlueprintMapLibrary.Map_Find` (`self.RoomRefs`) (`/Game/Player/Blueprints/BP_FP_Character.ActiveRoom` (`self.PlayerRef`)))) (- (`self.SongProgression`) 2)))
  (bind _output_2 (`|GetArrayItem` _keynotes (- (`self.SongProgression`) 2)))
  (bind _returnvalue_3 (+ _noteout -47))
  (bind (_days _hours _minutes _seconds _milliseconds) (`KismetMathLibrary.BreakTimespan` (- (`KismetMathLibrary.Now`) (+ _starttime _heldtime))))
  (if (== (`self.SongProgression`) 0)
    (set `self.SongProgression` 1))
  (set `self.SongTime` (+ (`self.SongTime`) (`GameplayStatics.GetWorldDeltaSeconds`)))
  (`/Game/Widgets/W_SongTimer.UpdateCursorPosition` (`/Game/Widgets/W_IngameMainUI.W_SongTimer` (`/Game/Player/Blueprints/BP_FP_Character.UI_Ref` (`self.PlayerRef`))) (/ (`self.SongTime`) (`self.TotalPlayLength`)))
  (if (> (`self.SongTime`) (* (`self.SongProgression`) (/ (`self.TotalPlayLength`) 4.0)))
    (`/Engine/EditorBlueprintResources/StandardMacros.IncrementInt` (`self.SongProgression`)
      (:`  `
        (if (== (`self.CurrentCheckForKeynoteTimer`) 0.0) :!label _label
          (set `local.IndexToCheck` (`KismetMathLibrary.SelectInt` 0 (- _returnvalue 1) (== _returnvalue 0)))
          (if (< (+ _milliseconds (* _seconds 1000)) (`KismetMathLibrary.FTrunc` (* (`self.MaxCheckForKeynoteTimer`) 1000.0))) :!label _label_2
            (if (== _noteout (+ _output_2 47))
              (`self.AddUsedNote` _output_2)
              (`self.ResetAttemptedNotes` :!label _label_3)
              (set `self.CurrentCheckForKeynoteTimer` 0.0)
              (if (>= (`self.SongProgression`) 5)
                (`self.ResetRitual`)
                (`/Game/Player/Blueprints/BP_FP_Character.RemoteTriggerToggleKeyboard` _playerref)
                (bind _returnvalue_4 (`KismetArrayLibrary.Array_Add` (`self.FinishedRooms`) _activeroom))
                (`/Game/Game/BP_RoomDivider.FinishedRitual` (`BlueprintMapLibrary.Map_Find` (`self.RoomRefs`) _activeroom))
                (if (== _returnvalue_4 2)
                  (`self.SwitchLighting`)
                  (elif (== _returnvalue_4 0)
                    (`/Game/Player/Blueprints/BP_FP_Character.GameEndEvent` (`self.PlayerRef`)))))
              (else
                (for _array_element _keynotes
                  (if (== _array_element _returnvalue_3)
                    (`self.AddAttemptedNote` _returnvalue_3)
                    (break)))
                (if (> _returnvalue_2 0)
                  (set `local.IndexToCheck` _returnvalue_2)
                  (goto _label_2)
                  (else
                    (`self.FailedSegment`)))))
            (else
              (bind _values (`BlueprintMapLibrary.Map_Values` (`self.PlayingNotes`)))
              (for _array_element_2 _values
                (bind (_note_2 _octave_2) (break `/Game/Game/Utilities/S_NoteInfo` _array_element_2))
                (bind _noteout_2 (`self.NoteOctaveToNote` _note_2 _octave_2))
                (if (== _noteout_2 (+ _output 47))
                  (set `local.IsPlayingKeynote` true)
                  (`self.AddUsedNote` _output)
                  (break)
                  (else
                    (for _array_element_3 (`/Game/Game/BP_RoomDivider.Keynotes` (`BlueprintMapLibrary.Map_Find` (`self.RoomRefs`) (`/Game/Player/Blueprints/BP_FP_Character.ActiveRoom` (`self.PlayerRef`))))
                      (bind _returnvalue_5 (- _noteout_2 47))
                      (if (== _array_element_3 _returnvalue_5)
                        (`self.AddAttemptedNote` _returnvalue_5)
                        (break))))))
              (if (`local.IsPlayingKeynote`)
                (goto _label_3)
                (else
                  (`self.FailedSegment`)))))
          (else
            (set `self.CurrentCheckForKeynoteTimer` (`KismetMathLibrary.FMin` (+ (`self.CurrentCheckForKeynoteTimer`) (`GameplayStatics.GetWorldDeltaSeconds`)) (`self.MaxCheckForKeynoteTimer`)))))))
    (elif (not (== (`self.CurrentCheckForKeynoteTimer`) 0.0))
      (goto _label))))

(fn `ResetAttemptedNotes`
  (bind _currentattemptedkeynotes (`self.CurrentAttemptedKeynotes`))
  (for _array_element _currentattemptedkeynotes
    (bind _asbp_fp_character (cast `/Game/Player/Blueprints/BP_FP_Character` (`GameplayStatics.GetPlayerPawn` 0)))
    (`/Game/Widgets/W_KeyboardInterface.InvalidateKeyNote` (`/Game/Widgets/W_IngameMainUI.W_KeyboardInterface` (`/Game/Player/Blueprints/BP_FP_Character.UI_Ref` _asbp_fp_character)) _array_element true true))
  (`KismetArrayLibrary.Array_Clear` _currentattemptedkeynotes))

(fn `ResetRitual`
  (bind _values (`BlueprintMapLibrary.Map_Values` (`self.PlayingNotes`)))
  (for _array_element _values
    (bind (_note _octave) (break `/Game/Game/Utilities/S_NoteInfo` _array_element))
    (`self.StopPlayingNote` (`self.NoteOctaveToNote` _note _octave) false true))
  (set `self.IsPlaying` false)
  (set `self.SongProgression` 0)
  (set `self.SongTime` 0.0)
  (set `self.CurrentCheckForKeynoteTimer` 0.0)
  (`/Game/Widgets/W_SongTimer.UpdateCursorPosition` (`/Game/Widgets/W_IngameMainUI.W_SongTimer` (`/Game/Player/Blueprints/BP_FP_Character.UI_Ref` (`self.PlayerRef`))) 0.0)
  (`BlueprintMapLibrary.Map_Clear` (`self.NoteHistory`))
  (`KismetArrayLibrary.Array_Clear` (`self.CurrentUsedKeynotes`))
  (`KismetArrayLibrary.Array_Clear` (`self.CurrentAttemptedKeynotes`)))

(fn `SoundReachedThreshhold`
  (params (PlayingSoundWave :type "SoundWave Object Reference") (PlaybackPercent :type "Float (single-precision)"))
  (locals (NoteWasJustAdded :type Boolean) (JustAddedNote :type "/Game/Game/Utilities/S_NoteInfo Structure"))
  (if (>= PlaybackPercent 0.8)
    (bind _values (`BlueprintMapLibrary.Map_Values` (`self.PlayingNotes`)))
    (for _array_element _values
      (bind (_note _octave _soundset _soundwave) (break `/Game/Game/Utilities/S_NoteInfo` _array_element))
      (if (== _soundwave PlayingSoundWave)
        (for _array_element_2 (`self.JustAddedNotes`)
          (if (== (`.SpawnedOrder_23_6FD0F84D4D9E1B08C5D8538F50475E8B` (break `/Game/Game/Utilities/S_NoteInfo` _array_element_2)) (`.SpawnedOrder_23_6FD0F84D4D9E1B08C5D8538F50475E8B` (break `/Game/Game/Utilities/S_NoteInfo` _array_element)))
            (set `local.NoteWasJustAdded` true)
            (set `local.JustAddedNote` _array_element_2)
            (break)))
        (if (`local.NoteWasJustAdded`)
          (`KismetArrayLibrary.Array_RemoveItem` (`self.JustAddedNotes`) _array_element_2)
          (else
            (`KismetArrayLibrary.Array_Add` (`self.FadingNotes`) _array_element)
            (`BlueprintMapLibrary.Map_Remove` (`self.PlayingNotes`) (`self.NoteOctaveToNote` _note _octave))
            (bind _asbp_fp_character (cast `/Game/Player/Blueprints/BP_FP_Character` (`GameplayStatics.GetPlayerPawn` 0)))
            (`/Game/Widgets/W_KeyboardInterface.ToggleButtonPressed` (`/Game/Widgets/W_IngameMainUI.W_KeyboardInterface` (`/Game/Player/Blueprints/BP_FP_Character.UI_Ref` _asbp_fp_character)) _array_element false)))))))

(fn `StartPlayingNote`
  (params (Note :type Integer) (Velocity :type Integer) (InputFromKeyboard :type Boolean))
  (locals (CurrentNote :type "/Game/Game/Utilities/S_NoteInfo Structure") (IsAlreadyPlaying :type Boolean))
  (bind _currentnote (`local.CurrentNote`))
  (bind _basevolumedivider (`self.BaseVolumeDivider`))
  (bind _currenthighestorder (`self.CurrentHighestOrder`))
  (set `self.IsPlaying` true)
  (if (`self.KeyboardIsShown`)
    (bind _values (`BlueprintMapLibrary.Map_Values` (`self.PlayingNotes`)))
    (for _array_element _values
      (bind (_note _octave) (break `/Game/Game/Utilities/S_NoteInfo` _array_element))
      (if (== Note (`self.NoteOctaveToNote` _note _octave))
        (set `local.IsAlreadyPlaying` true)
        (break)))
    (if (not (`local.IsAlreadyPlaying`))
      (bind _returnvalue (`|GetDataTableRow` (select `/Game/Game/Utilities/E_Soundset` (`self.ActiveSoundset`) :`NewEnumerator3` "/Game/Game/Utilities/DefaultNoteInfos/DT_DefaultNoteInfo_Celeste.DT_DefaultNoteInfo_Celeste" :`NewEnumerator4` "/Game/Game/Utilities/DefaultNoteInfos/DT_DefaultNoteInfo_Glockenspiel.DT_DefaultNoteInfo_Glockenspiel" :`NewEnumerator5` "/Game/Game/Utilities/DefaultNoteInfos/DT_DefaultNoteInfo_MusicBox.DT_DefaultNoteInfo_MusicBox" :`NewEnumerator6` "/Game/Game/Utilities/DefaultNoteInfos/DT_DefaultNoteInfo_Organ.DT_DefaultNoteInfo_Organ" :`NewEnumerator7` "/Game/Game/Utilities/DefaultNoteInfos/DT_DefaultNoteInfo_Piano.DT_DefaultNoteInfo_Piano" :!type "DataTable Object Reference") (`KismetStringLibrary.Conv_StringToName` (`KismetStringLibrary.Conv_IntToString` Note)))
        (:`then`
          (set `local.CurrentNote` _returnvalue)
          (bind _returnvalue_2 (`GameplayStatics.CreateSound2D` (`.SoundWave_17_4A934C2C484FC600EE6D1380D70E89E3` (break `/Game/Game/Utilities/S_NoteInfo` _returnvalue)) (* 1 (+ (* (/ Velocity 127) (/ (- _basevolumedivider 1.0) _basevolumedivider)) (/ 1.0 _basevolumedivider))) 1.0 0.0 null))
          (setmembers `/Game/Game/Utilities/S_NoteInfo` :`StructRef` _currentnote :`SpawnedOrder` _currenthighestorder :`StartTime` (`KismetMathLibrary.Now`) :`AudioRef` _returnvalue_2 :`IsKeyboardInput` InputFromKeyboard)
          (`/Engine/EditorBlueprintResources/StandardMacros.IncrementInt` _currenthighestorder
            (:`  `
              (add `AudioComponent.OnAudioPlaybackPercent` _returnvalue_2 (`|CreateDelegate` :!event `SoundReachedThreshhold`))
              (`BlueprintMapLibrary.Map_Add` (`self.PlayingNotes`) Note _currentnote)
              (`KismetArrayLibrary.Array_Add` (`self.JustAddedNotes`) _currentnote)
              (`AudioComponent.Play` _returnvalue_2 0.0)
              (`/Game/Game/NoteBarRendering/BP_NotebarRenderer.StartSoundBar` (`self.NotebarRendererRef`) _currentnote)
              (bind _asbp_fp_character (cast `/Game/Player/Blueprints/BP_FP_Character` (`GameplayStatics.GetPlayerPawn` 0)))
              (`/Game/Widgets/W_KeyboardInterface.ToggleButtonPressed` (`/Game/Widgets/W_IngameMainUI.W_KeyboardInterface` (`/Game/Player/Blueprints/BP_FP_Character.UI_Ref` _asbp_fp_character)) _currentnote true))))))))

(fn `StopPlayingNote`
  (params (Note :type Integer) (InputFromKeyboard :type Boolean) (Force :type Boolean))
  (locals (CurrentNote :type Integer) (IsCorrectInputMethod :type Boolean))
  (bind _notehistory (`self.NoteHistory`))
  (bind (_value _returnvalue) (`BlueprintMapLibrary.Map_Find` (`self.PlayingNotes`) (`local.CurrentNote`)))
  (bind (_note _octave _soundset _soundwave _spawnedorder _starttime _heldtime _audioref) (break `/Game/Game/Utilities/S_NoteInfo` _value))
  (bind _output_get (set `local.CurrentNote` Note))
  (if (`self.KeyboardIsShown`)
    (bind _values (`BlueprintMapLibrary.Map_Values` (`self.PlayingNotes`)))
    (for _array_element _values
      (bind (_note_2 _octave_2 _soundset_2 _soundwave_2 _spawnedorder_2 _starttime_2 _heldtime_2 _audioref_2 _iskeyboardinput) (break `/Game/Game/Utilities/S_NoteInfo` _array_element))
      (if (and (== _output_get (`self.NoteOctaveToNote` _note_2 _octave_2)) (or (== _iskeyboardinput InputFromKeyboard) Force))
        (set `local.IsCorrectInputMethod` true)
        (break)))
    (if (`local.IsCorrectInputMethod`)
      (if _returnvalue
        (`/Engine/EditorBlueprintResources/StandardMacros.IsValid` _audioref
          (:`Is Valid`
            (clear `AudioComponent.OnAudioPlaybackPercent` _audioref)
            (`/Game/Game/NoteBarRendering/BP_NotebarRenderer.StopSoundbar` (`self.NotebarRendererRef`) _value)
            (bind _asbp_fp_character (cast `/Game/Player/Blueprints/BP_FP_Character` (`GameplayStatics.GetPlayerPawn` 0)))
            (`/Game/Widgets/W_KeyboardInterface.ToggleButtonPressed` (`/Game/Widgets/W_IngameMainUI.W_KeyboardInterface` (`/Game/Player/Blueprints/BP_FP_Character.UI_Ref` _asbp_fp_character)) _value false)
            (bind _structout (setmembers `/Game/Game/Utilities/S_NoteInfo` :`StructRef` _value :`HeldTime` (- (`KismetMathLibrary.Now`) (`.StartTime_10_E76DBD95483935FB488B5F86CEB59283` (break `/Game/Game/Utilities/S_NoteInfo` _value)))))
            (`BlueprintMapLibrary.Map_Add` _notehistory (`BlueprintMapLibrary.Map_Length` _notehistory) _structout)
            (`KismetArrayLibrary.Array_Add` (`self.FadingNotes`) _structout)
            (`BlueprintMapLibrary.Map_Remove` (`self.PlayingNotes`) (`local.CurrentNote`))))))))

(fn `UserConstructionScript`)