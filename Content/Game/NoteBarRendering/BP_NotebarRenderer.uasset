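; BP_NotebarRenderer is an actor that visualises played notes as BP_Soundbar bars laid out like piano keys.
; StartSoundBar spawns a bar at an X offset chosen by note and octave, with per-note positions only for octave options 2 and 3.
; Tick stretches held bars along Y until StopSoundbar releases them, matching SpawnedOrder across parallel note and bar arrays.
; Bars leaving the Box volume are destroyed.
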(event `self.ReceiveTick`
  (params (DeltaSeconds :type "Float (single-precision)"))
  (for _array_element (`self.ActiveSoundbars`)
    (bind _soundbar (`/Game/Game/NoteBarRendering/BP_Soundbar.Soundbar` _array_element))
    (`SceneComponent.SetWorldScale3D` _soundbar (`KismetMathLibrary.MakeVector` (.x (`SceneComponent.K2_GetComponentScale` _soundbar)) (+ (.y (`SceneComponent.K2_GetComponentScale` _soundbar)) (* DeltaSeconds 250.0)) (.z (`SceneComponent.K2_GetComponentScale` _soundbar))))))

(event `self.Box.OnComponentEndOverlap`
  (params (OverlappedComponent :type "PrimitiveComponent Object Reference") (OtherActor :type "Actor Object Reference") (OtherComp :type "PrimitiveComponent Object Reference") (OtherBodyIndex :type Integer))
  (bind _asbp_soundbar (cast `/Game/Game/NoteBarRendering/BP_Soundbar` OtherActor))
  (`self.K2_DestroyActor` _asbp_soundbar))

(fn `StartSoundBar`
  (params (NoteInfo :type "/Game/Game/Utilities/S_NoteInfo Structure"))
  (bind (_note _octave) (break `/Game/Game/Utilities/S_NoteInfo` NoteInfo))
  (`KismetArrayLibrary.Array_Add` (`self.ActiveNotes`) NoteInfo)
  (bind _returnvalue (`|SpawnActorFromClass` "/Game/Game/NoteBarRendering/BP_Soundbar.BP_Soundbar_C" (`KismetMathLibrary.MakeTransform` (`KismetMathLibrary.MakeVector` (+ (.x (`self.K2_GetActorLocation`)) (select `int` _octave :`0` 0.0 :`1` 0.0 :`2` (select `/Game/Game/Utilities/E_Notes` _note :`NewEnumerator0` -700.0 :`NewEnumerator1` -650.0 :`NewEnumerator2` -600.0 :`NewEnumerator3` -550.0 :`NewEnumerator4` -500.0 :`NewEnumerator5` -400.0 :`NewEnumerator6` -350.0 :`NewEnumerator7` -300.0 :`NewEnumerator8` -250.0 :`NewEnumerator9` -200.0 :`NewEnumerator13` -150.0 :`NewEnumerator10` -100.0) :`3` (select `/Game/Game/Utilities/E_Notes` _note :`NewEnumerator1` 50.0 :`NewEnumerator2` 100.0 :`NewEnumerator3` 150.0 :`NewEnumerator4` 200.0 :`NewEnumerator5` 300.0 :`NewEnumerator6` 350.0 :`NewEnumerator7` 400.0 :`NewEnumerator8` 450.0 :`NewEnumerator9` 500.0 :`NewEnumerator13` 550.0 :`NewEnumerator10` 600.0) :`4` 700.0)) (.y (`self.K2_GetActorLocation`)) (.z (`self.K2_GetActorLocation`)))) "Undefined" "MultiplyWithRoot" null null))
  (`KismetArrayLibrary.Array_Add` (`self.ActiveSoundbars`) _returnvalue))

(fn `StopSoundbar`
  (params (NoteInfo :type "/Game/Game/Utilities/S_NoteInfo Structure"))
  (for (_array_element _array_index) (`self.ActiveNotes`)
    (if (== (`.SpawnedOrder_23_6FD0F84D4D9E1B08C5D8538F50475E8B` (break `/Game/Game/Utilities/S_NoteInfo` _array_element)) (`.SpawnedOrder_23_6FD0F84D4D9E1B08C5D8538F50475E8B` (break `/Game/Game/Utilities/S_NoteInfo` NoteInfo)))
      (set `/Game/Game/NoteBarRendering/BP_Soundbar.IsBeingHeld` false (`|GetArrayItem` (`self.ActiveSoundbars`) _array_index))
      (`KismetArrayLibrary.Array_Remove` (`self.ActiveSoundbars`) _array_index)
      (`KismetArrayLibrary.Array_Remove` (`self.ActiveNotes`) _array_index)
      (break))))

(fn `UserConstructionScript`)