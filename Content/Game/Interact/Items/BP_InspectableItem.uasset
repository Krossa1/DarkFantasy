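; Interactable physics prop that the player pulls up to the camera to inspect, rotate (unless it is paper) and search for notes.
; A reversible Timeline moves the mesh to and from view while input mapping contexts swap.
; Clicks sphere-trace toward the cursor to collect tagged notes, retexturing paper items, or just play fake-note sounds.
; Construction optionally attaches a BP_Note child; Respawn restores the starting transform, and SpawnDuplicate's logic is disconnected.
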(event `RotateInspect`
  (params (EventStarted :type Boolean))
  ; Inspect Input
  ;; Check if Rotating
  (if (`self.isPaper`)
    _
    (elif EventStarted
      (if (`self.IsInspecting`)
        (set `self.Rotate?` true))
      (elif (`self.IsInspecting`)
        (set `self.Rotate?` false)))))

(event `self.ReceiveBeginPlay`
  ; Set Inital Location on BeginPlay
  (set `self.InitialTransform` (`KismetMathLibrary.Conv_VectorToTransform` (`SceneComponent.K2_GetComponentLocation` (`self.StaticMesh`)))))

(event `InspectCollect`
  ; Inspect Input
  ;; Check for Note
  (if (`self.IsInspecting`)
    (bind _outhits (`KismetSystemLibrary.SphereTraceMulti` :`Start` (`SceneComponent.K2_GetComponentLocation` (`/Game/Player/Blueprints/BP_FP_Character.Camera` (`self.Player`))) :`End` (`.Location` (`GameplayStatics.BreakHitResult` (`PlayerController.GetHitResultUnderCursorByChannel` (`GameplayStatics.GetPlayerController` 0) "TraceTypeQuery1" true))) :`Radius` 3.0 :`TraceChannel` "TraceTypeQuery1" :`DrawDebugType` "ForDuration"))
    (for _array_element _outhits
      (bind (_bblockinghit _binitialoverlap _time _distance _location _impactpoint _normal _impactnormal _physmat _hitactor) (`GameplayStatics.BreakHitResult` _array_element))
      (if (`self.ActorHasTag` _hitactor "Note")
        (bind _asbp_note (cast `/Game/Game/NoteSystem/BP_Note` _hitactor))
        (`/Game/Game/NoteSystem/BP_Note.PlaySound` _asbp_note)
        (`/Game/Player/Blueprints/BP_FP_Character.CollectNote` (`self.Player`) _hitactor)
        (if (`self.isPaper`)
          (bind _returnvalue (`PrimitiveComponent.CreateDynamicMaterialInstance` (`self.StaticMesh`) 0 "/Game/Art/Material_001.Material_001" "None"))
          (`MaterialInstanceDynamic.SetTextureParameterValue` _returnvalue "DiffuseColorMap" "/Game/Art/briefTest.briefTest"))
        (elif (`self.ActorHasTag` _hitactor "FakeNote")
          (bind _asbp_note_2 (cast `/Game/Game/NoteSystem/BP_Note` _hitactor))
          (`/Game/Game/NoteSystem/BP_Note.PlaySound` _asbp_note_2))))))

(event `EnhancedInput|/Game/Player/InputMappings/Actions/IA_Interact`
  (params (ActionValue :type Boolean) (ElapsedSeconds :type "Float (double-precision)") (TriggeredSeconds :type "Float (double-precision)") (InputAction :type "InputAction Object Reference" :default "/Game/Player/InputMappings/Actions/IA_Interact.IA_Interact")))

(event `/Game/Game/Interact/BPI_InteractInterface.OnInteract`
  (params (Player :type "/Game/Player/Blueprints/BP_FP_Character Object Reference"))
  (bind _returnvalue (`GameplayStatics.GetPlayerController` 0))
  (bind _player (`self.Player`))
  (bind _staticmesh (`self.StaticMesh`))
  (bind (_lastposition_location _lastposition_rotation) (`KismetMathLibrary.BreakTransform` (`self.LastPosition`)))
  (bind _returnvalue_2 (pcsubsystem `EnhancedInputLocalPlayerSubsystem` _returnvalue))
  (bind (_returnvalue_location _returnvalue_rotation) (`KismetMathLibrary.BreakTransform` (`SceneComponent.K2_GetComponentToWorld` (`/Game/Player/Blueprints/BP_FP_Character.ImspectRef` _player))))
  ; Start Interacting
  (`PrimitiveComponent.SetSimulatePhysics` _staticmesh false)
  (`PrimitiveComponent.SetCollisionEnabled` _staticmesh "QueryOnly")
  (set `self.Player` Player)
  (`WidgetBlueprintLibrary.SetInputMode_GameAndUIEx` (`GameplayStatics.GetPlayerController` 0) null)
  (set `self.LastPosition` (`KismetMathLibrary.Conv_VectorToTransform` (`SceneComponent.K2_GetComponentLocation` (`self.StaticMesh`))))
  (`EnhancedInputSubsystemInterface.RemoveMappingContext` _returnvalue_2 "/Game/Player/InputMappings/IMC_DefaultContext.IMC_DefaultContext" (struct))
  (set `/Game/Player/Blueprints/BP_FP_Character.CurrentInspectItem` self (`self.Player`))
  (`EnhancedInputSubsystemInterface.AddMappingContext` _returnvalue_2 "/Game/Player/InputMappings/IMC_InspectContext.IMC_InspectContext" 0 (struct))
  (set `PlayerController.bShowMouseCursor` true _returnvalue)
  (set `self.isReversing` false)
  (bind (_direction _newtrack_0) (`Timeline|Timeline` :!label _label)
    (:`Update`
      (`SceneComponent.K2_SetWorldTransform` (`self.StaticMesh`) (`KismetMathLibrary.MakeTransform` (`KismetMathLibrary.VLerp` _lastposition_location (+ _returnvalue_location (* (`SceneComponent.GetForwardVector` (`/Game/Player/Blueprints/BP_FP_Character.Camera` _player)) (`self.InspectDistance`))) _newtrack_0) (`KismetMathLibrary.RLerp` _lastposition_rotation _returnvalue_rotation _newtrack_0) (`self.ItemScale`)) false false)
      (set `self.IsInspecting` true)
      (`SceneComponent.SetVisibility` (`self.Widget`) false false))
    (:`Finished`
      ; Stop Interacting
      (if (`self.isReversing`)
        (`PrimitiveComponent.SetCollisionEnabled` (`self.StaticMesh`) "QueryAndPhysics")
        (`PrimitiveComponent.SetSimulatePhysics` (`self.StaticMesh`) true)
        (`SceneComponent.SetVisibility` (`self.Widget`) true false)))))

(event `RotateX`
  (params (AxisValue :type "Float (double-precision)"))
  ; Inspect Input
  ;; Set Mouse Movement Horizontally
  (if (`self.Rotate?`)
    (`SceneComponent.K2_AddLocalRotation` (`self.StaticMesh`) (`KismetMathLibrary.MakeRotator` (* AxisValue -1.0)) false false)))

(event `RotateY`
  (params (`Axis Value` :type "Float (double-precision)"))
  ; Inspect Input
  ;; Set Mouse Movement Vertically
  (if (`self.Rotate?`)
    (`SceneComponent.K2_AddLocalRotation` (`self.StaticMesh`) (`KismetMathLibrary.MakeRotator` 0.0 (* 1.0 `Axis Value`)) false false)))

(event `LeaveInspect`
  (bind _returnvalue (`GameplayStatics.GetPlayerController` 0))
  (bind _returnvalue_2 (pcsubsystem `EnhancedInputLocalPlayerSubsystem` (`GameplayStatics.GetPlayerController` 0)))
  ; Stop Interacting
  (if (`self.IsInspecting`)
    (set `PlayerController.bShowMouseCursor` false _returnvalue)
    (`WidgetBlueprintLibrary.SetInputMode_GameOnly` _returnvalue)
    (set `self.IsInspecting` false)
    (`EnhancedInputSubsystemInterface.RemoveMappingContext` _returnvalue_2 "/Game/Player/InputMappings/IMC_InspectContext.IMC_InspectContext" (struct))
    (set `/Game/Player/Blueprints/BP_FP_Character.CurrentInspectItem` null (`self.Player`))
    (`EnhancedInputSubsystemInterface.AddMappingContext` _returnvalue_2 "/Game/Player/InputMappings/IMC_DefaultContext.IMC_DefaultContext" 0 (struct))
    (set `self.isReversing` true)
    (goto _label :!via `Reverse`)))

(event `Respawn`
  (bind (_initialtransform_location _initialtransform_rotation _initialtransform_scale) (`KismetMathLibrary.BreakTransform` (`self.InitialTransform`)))
  (`PrimitiveComponent.SetSimulatePhysics` (`self.StaticMesh`) false)
  (`SceneComponent.K2_SetWorldTransform` (`self.StaticMesh`) (`KismetMathLibrary.MakeTransform` _initialtransform_location _initialtransform_rotation _initialtransform_scale) false false)
  (`KismetSystemLibrary.Delay` 1.0)
  (`PrimitiveComponent.SetSimulatePhysics` (`self.StaticMesh`) true))

(fn `ReturnToInitialPosition`
  (`self.K2_SetActorTransform` (`self.LastPosition`) false true)
  (`PrimitiveComponent.SetSimulatePhysics` (`self.StaticMesh`) true)
  (`PrimitiveComponent.SetEnableGravity` (`self.StaticMesh`) true))

(fn `SpawnDuplicate`
  (params (CamRef :type "SceneCaptureComponent2D Object Reference") (DuplicateTransform :type "Transform Structure")))

(fn `UpdateDuplicate`
  (`self.K2_SetActorRotation` (`self.DuplicateRef`) (`self.K2_GetActorRotation`) false))

(fn `UserConstructionScript`
  (`parent.UserConstructionScript`)
  (if (`self.HasNote`)
    (`ChildActorComponent.SetChildActorClass` (`self.ChildActor`) "/Game/Game/NoteSystem/BP_Note.BP_Note_C")
    (`SceneComponent.K2_SetRelativeTransform` (`self.ChildActor`) (`self.NoteTransform`) false false)
    (bind _asbp_note (cast `/Game/Game/NoteSystem/BP_Note` (`ChildActorComponent.ChildActor` (`self.ChildActor`))))
    (set `/Game/Game/NoteSystem/BP_Note.NoteOctave` (`self.NoteOctave`) _asbp_note)
    (else
      (`ChildActorComponent.SetChildActorClass` (`self.ChildActor`) null))))