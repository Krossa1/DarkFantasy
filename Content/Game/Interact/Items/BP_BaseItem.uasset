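; BP_BaseItem is a base interactable item that shows an interact prompt when the player comes near.
; Its construction script applies configurable mesh, scale, sphere radii and icon position, plus optional debug visibility for the spheres.
; The inner sphere creates a W_Interact widget and animates it in, then on exit reverses it, clears the mesh overlay and removes it.
; Older icon logic remains: the outer sphere only hides its icon, and inner icon toggles are unwired.
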(event `self.InnerSqhereCollision.OnComponentBeginOverlap`
  (params (OverlappedComponent :type "PrimitiveComponent Object Reference") (OtherActor :type "Actor Object Reference") (OtherComp :type "PrimitiveComponent Object Reference") (OtherBodyIndex :type Integer) (bFromSweep :type Boolean) (SweepResult :type "HitResult Structure (by ref)"))
  (bind _widget (`self.Widget`))
  ; Show Interact Icon
  (if (== OtherActor (`GameplayStatics.GetPlayerCharacter` 0))
    (bind _returnvalue (`|CreateWidget` "/Game/Widgets/W_Interact.W_Interact_C"))
    (bind _output_get (set `self.InteractWidget` _returnvalue))
    (`WidgetComponent.SetWidget` _widget _output_get)
    (`SceneComponent.SetVisibility` _widget true false)
    (bind _interactwidget (`self.InteractWidget`)
      (:`then`
        (`/Game/Widgets/W_Interact.ToggleItem` _interactwidget true)
        (if (not (`self.HintVisible`))
          (`UserWidget.PlayAnimation` _interactwidget (`/Game/Widgets/W_Interact.ShowInteract` _interactwidget) 0.0 1 "Forward" 1.5 false)
          (set `self.HintVisible` true)))
      (:`else`))))

(event `self.InnerSqhereCollision.OnComponentEndOverlap`
  (params (OverlappedComponent :type "PrimitiveComponent Object Reference") (OtherActor :type "Actor Object Reference") (OtherComp :type "PrimitiveComponent Object Reference") (OtherBodyIndex :type Integer))
  ; Show Interact Icon
  (if (== (`GameplayStatics.GetPlayerCharacter` 0) OtherActor)
    (bind _interactwidget (`self.InteractWidget`)
      (:`then`
        (if (`self.HintVisible`)
          (`UserWidget.PlayAnimation` _interactwidget (`/Game/Widgets/W_Interact.ShowInteract` _interactwidget) 0.0 1 "Reverse" 1.5 false)
          (set `self.HintVisible` false))
        (`MeshComponent.SetOverlayMaterial` (`self.StaticMesh`) null)
        (`KismetSystemLibrary.Delay` 0.2)
        (`Widget.RemoveFromParent` (`self.InteractWidget`))
        (set `self.InteractWidget` null)
        (`SceneComponent.SetVisibility` (`self.Widget`) false false))
      (:`else`))))

(event `self.OuterSphereCollision.OnComponentBeginOverlap`
  (params (OverlappedComponent :type "PrimitiveComponent Object Reference") (OtherActor :type "Actor Object Reference") (OtherComp :type "PrimitiveComponent Object Reference") (OtherBodyIndex :type Integer) (bFromSweep :type Boolean) (SweepResult :type "HitResult Structure (by ref)"))
  ; Show Icons (Old)
  (if (== OtherActor (`GameplayStatics.GetPlayerCharacter` 0))
    (`SceneComponent.SetVisibility` (`self.OuterIcon`) false false)))

(event `self.OuterSphereCollision.OnComponentEndOverlap`
  (params (OverlappedComponent :type "PrimitiveComponent Object Reference") (OtherActor :type "Actor Object Reference") (OtherComp :type "PrimitiveComponent Object Reference") (OtherBodyIndex :type Integer))
  ; Show Icons (Old)
  (if (== (`GameplayStatics.GetPlayerCharacter` 0) OtherActor)
    (`SceneComponent.SetVisibility` (`self.OuterIcon`) false false)))

(fn `UserConstructionScript`
  (bind _staticmesh (`self.StaticMesh`))
  (`|ExecutionSequence`
    (:`then_0`
      ; Set Spheres
      (`SphereComponent.SetSphereRadius` (`self.InnerSqhereCollision`) (`self.Inner Sphere Radius`) true)
      (`SphereComponent.SetSphereRadius` (`self.OuterSphereCollision`) (`self.Outer Sphere Radius`) true)
      ; Set Icon Location
      (`SceneComponent.K2_SetRelativeLocation` (`self.InnerIcon`) (`self.Icon Location`) false false)
      (`SceneComponent.K2_SetRelativeLocation` (`self.OuterIcon`) (`self.Icon Location`) false false))
    (:`then_1`
      ; Setting Mesh Dynamically
      (`StaticMeshComponent.SetStaticMesh` (`self.StaticMesh`) (`self.ItemMesh`))
      ; Setting Mesh Scale Dynamically
      (`SceneComponent.K2_SetWorldTransform` _staticmesh (`KismetMathLibrary.MakeTransform` (`SceneComponent.K2_GetComponentLocation` _staticmesh) (`SceneComponent.K2_GetComponentRotation` _staticmesh) (`self.ItemScale`)) false false))
    (:`then_2`
      ; Debugging
      (if (`self.Debugging?`)
        (`SceneComponent.SetVisibility` (`self.InnerSqhereCollision`) true false)
        (`SceneComponent.SetVisibility` (`self.OuterSphereCollision`) true false)
        (else
          (`SceneComponent.SetVisibility` (`self.InnerSqhereCollision`) false false)
          (`SceneComponent.SetVisibility` (`self.OuterSphereCollision`) false false))))))