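; BP_RoomDivider is a single or double door between rooms that tracks the player character's active room.
; When an overlap with ForwardBox ends, BackwardBox overlap determines the player's direction and sets ActiveRoom.
; The first forward exit also calls ToggleDoor, whose timeline swings the doors between closed yaw and their BeginPlay rotations.
; The construction script applies one shared mesh to both leaves.
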(event `self.ReceiveBeginPlay`
  (set `self.LeftDoorInitialZRotation` (.yaw (`SceneComponent.RelativeRotation` (`self.Door_L`))))
  (set `self.RightDoorInitialZRotation` (.yaw (`SceneComponent.RelativeRotation` (`self.Door_R`)))))

(event `ToggleDoor`
  (bind _closeddooryaw (`self.ClosedDoorYaw`))
  (bind _output_get (set `self.DoorOpen` (not (`self.DoorOpen`))))
  (if _output_get
    (bind (_direction _progress) (`Timeline|RotateDoor` :!label _label)
      (:`Update`
        (`SceneComponent.K2_SetRelativeRotation` (`self.Door_L`) (`KismetMathLibrary.RLerp` (`KismetMathLibrary.MakeRotator` 0.0 0.0 _closeddooryaw) (`KismetMathLibrary.MakeRotator` 0.0 0.0 (`self.LeftDoorInitialZRotation`)) _progress true) true false)
        (if (`self.IsDoubleDoor`)
          (`SceneComponent.K2_SetRelativeRotation` (`self.Door_R`) (`KismetMathLibrary.RLerp` (`KismetMathLibrary.MakeRotator` 0.0 0.0 (+ _closeddooryaw 180.0)) (`KismetMathLibrary.MakeRotator` 0.0 0.0 (`self.RightDoorInitialZRotation`)) _progress true) true false))))
    (else
      (goto _label :!via `ReverseFromEnd`))))

(event `self.ForwardBox.OnComponentEndOverlap`
  (params (OverlappedComponent :type "PrimitiveComponent Object Reference") (OtherActor :type "Actor Object Reference") (OtherComp :type "PrimitiveComponent Object Reference") (OtherBodyIndex :type Integer))
  (`self.ExitedCollision`))

(fn `ExitedCollision`
  (bind _asbp_fp_character (cast `/Game/Player/Blueprints/BP_FP_Character` (`GameplayStatics.GetPlayerPawn` 0)))
  (if (not (`PrimitiveComponent.IsOverlappingActor` (`self.BackwardBox`) _asbp_fp_character))
    (set `/Game/Player/Blueprints/BP_FP_Character.ActiveRoom` (`self.ForwardRoom`) _asbp_fp_character)
    (if (not (`self.HasEntered`))
      (set `self.HasEntered` true)
      (`self.ToggleDoor`))
    (else
      (set `/Game/Player/Blueprints/BP_FP_Character.ActiveRoom` "NewEnumerator1" _asbp_fp_character))))

(fn `UserConstructionScript`
  (bind _door_l (`self.Door_L`))
  (bind _doormesh_l (`self.DoorMesh_L`))
  (bind _door_r (`self.Door_R`))
  (`/Engine/EditorBlueprintResources/StandardMacros.IsValid` _doormesh_l
    (:`Is Valid`
      (`SceneComponent.SetWorldScale3D` _door_l (1.0 1.0 1.0))
      (`StaticMeshComponent.SetStaticMesh` _door_l _doormesh_l))
    (:`Is Not Valid`
      _))
  (if (`self.IsDoubleDoor`)
    (`SceneComponent.SetWorldScale3D` _door_r (1.0 1.0 1.0))
    (`StaticMeshComponent.SetStaticMesh` _door_r _doormesh_l)))