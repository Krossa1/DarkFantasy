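; BP_Respawning is a trigger actor that respawns inspectable items entering its collision component.
; On component overlap, it checks the other actor for BPI_InteractInterface, casts it to BP_InspectableItem and calls Respawn on it.
; A separate actor-overlap handler only prints debug text and casts to BP_BaseItem; its sole binding sits inside the handler itself, so nothing here initially binds it.
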(event `OnActorBeginOverlap_Event` :!signature `self.OnActorBeginOverlap`
  (params (OverlappedActor :type "Actor Object Reference") (OtherActor :type "Actor Object Reference"))
  (`KismetSystemLibrary.PrintText` "inevent")
  (add `self.OnActorBeginOverlap` (delegate `OnActorBeginOverlap_Event`))
  (bind _asbp_base_item (cast `/Game/Player/Blueprints/Interact/Items/BP_BaseItem` OverlappedActor))
  (`KismetSystemLibrary.PrintText` (`KismetTextLibrary.Conv_ObjectToText` _asbp_base_item)))

(event `self.CollisionComponent.OnComponentBeginOverlap`
  (params (OverlappedComponent :type "PrimitiveComponent Object Reference") (OtherActor :type "Actor Object Reference") (OtherComp :type "PrimitiveComponent Object Reference") (OtherBodyIndex :type Integer) (bFromSweep :type Boolean) (SweepResult :type "HitResult Structure (by ref)"))
  (if (`KismetSystemLibrary.DoesImplementInterface` OtherActor "/Game/Player/Blueprints/Interact/BPI_InteractInterface.BPI_InteractInterface_C")
    (`KismetSystemLibrary.PrintText` "inevent")
    (bind _asbp_inspectable_item (cast `/Game/Player/Blueprints/Interact/Items/BP_InspectableItem` OtherActor))
    (`/Game/Player/Blueprints/Interact/Items/BP_InspectableItem.Respawn` _asbp_inspectable_item)))

(fn `UserConstructionScript`)