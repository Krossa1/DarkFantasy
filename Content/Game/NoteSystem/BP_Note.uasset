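; BP_Note is a note actor from the note system with a collect sound, delayed destruction and an optional respawn.
; It plays its own sound or a default collect sound, and destroys itself after a very brief delay.
; The construction script stores only the mesh's world location as a transform.
; Respawn, when allowed, resets the mesh to that transform with physics off, then re-enables simulation after a short delay.
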(event `DestroyAfterDelay`
  (`KismetSystemLibrary.Delay` 0.05)
  (`self.K2_DestroyActor`))

(event `PlaySound`
  (`/Engine/EditorBlueprintResources/StandardMacros.IsValid` (`self.NoteSound`)
    (:`Is Valid`
      (`GameplayStatics.PlaySound2D` (`self.NoteSound`) 0.5 1.0 0.0 null null))
    (:`Is Not Valid`
      (`GameplayStatics.PlaySound2D` "/Game/Sound/GeneralSFX/DefaultCollect.DefaultCollect" 0.5 1.0 0.0 null null))))

(event `Respawn`
  (bind (_initial_transform_location _initial_transform_rotation _initial_transform_scale) (`KismetMathLibrary.BreakTransform` (`self.Initial Transform`)))
  (if (`self.CanRespawn?`)
    (`PrimitiveComponent.SetSimulatePhysics` (`self.StaticMesh1`) false)
    (`SceneComponent.K2_SetWorldTransform` (`self.StaticMesh1`) (`KismetMathLibrary.MakeTransform` _initial_transform_location _initial_transform_rotation _initial_transform_scale) false false)
    (`KismetSystemLibrary.Delay` 1.0)
    (`PrimitiveComponent.SetSimulatePhysics` (`self.StaticMesh1`) true)))

(fn `UserConstructionScript`
  (set `self.Initial Transform` (`KismetMathLibrary.Conv_VectorToTransform` (`SceneComponent.K2_GetComponentLocation` (`self.StaticMesh1`)))))