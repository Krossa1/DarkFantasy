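; Interactable door Blueprint that toggles between open and closed each time it is interacted with.
; It caches the mesh's relative rotation on BeginPlay and flips an Opened flag to play or reverse a timeline.
; The timeline alpha lerps the mesh yaw from its starting value to a quarter turn away.
; Timeline updates also trigger a short delay and a placeholder print noting that a can-interact check is still to be added.
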(event `self.ReceiveBeginPlay`
  (set `self.Starting Rotator ` (`SceneComponent.RelativeRotation` (`self.StaticMesh`))))

(event `/Game/Player/Blueprints/Interact/BPI_InteractInterface.OnInteract`
  (params (Player :type "/Game/Player/Blueprints/BP_FP_Character Object Reference"))
  (bind (_starting_rotator__roll _starting_rotator__pitch _starting_rotator__yaw) (`KismetMathLibrary.BreakRotator` (`self.Starting Rotator `)))
  (if (`self.Opened?`)
    (set `self.Opened?` false)
    (bind (_direction _alpha) (`Timeline|TM_InteractWIthDoor` :!via `Reverse` :!label _label)
      (:`Update`
        (`SceneComponent.K2_SetRelativeRotation` (`self.StaticMesh`) (`KismetMathLibrary.MakeRotator` _starting_rotator__roll _starting_rotator__pitch (`KismetMathLibrary.Lerp` _starting_rotator__yaw (- _starting_rotator__yaw 90.0) _alpha)) false false)
        (`KismetSystemLibrary.Delay` 0.2)
        (`KismetSystemLibrary.PrintText` "Add Can Interact")))
    (else
      (set `self.Opened?` true)
      (goto _label :!via `PlayFromStart`))))

(fn `UserConstructionScript`
  (`parent.UserConstructionScript`))