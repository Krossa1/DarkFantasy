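; Interactable item that the player can inspect, optionally carrying a BP_Note child actor built at construction.
; On interact it disables physics, enables note collision, saves its transform and hands itself to a spawned off-world BP_Inspecting; this path requires the note cast to succeed.
; It can spawn a hidden-mesh duplicate positioned relative to the player camera and mirror its rotation onto it.
; ReturnToInitialPosition detaches it, restores the transform and re-enables physics.
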(event `/Game/Player/Blueprints/Interact/BPI_InteractInterface.OnInteract`
  (params (Player :type "/Game/Player/Blueprints/BP_FP_Character Object Reference"))
  ; Inspect Item
  (if (`self.IsDuplicate`)
    _
    (elif (`self.Inspect?`)
      (bind _returnvalue (`|SpawnActorFromClass` "/Game/Player/Blueprints/Interact/BP_Inspecting.BP_Inspecting_C" (`KismetMathLibrary.MakeTransform` (10000.0 0.0 0.0)) "Undefined" "MultiplyWithRoot" null null))
      (`PrimitiveComponent.SetSimulatePhysics` (`self.StaticMesh`) false)
      (bind _asbp_note (cast `/Game/Player/Blueprints/NoteSystem/BP_Note` (`ChildActorComponent.ChildActor` (`self.ChildActor`))))
      (`PrimitiveComponent.SetCollisionProfileName` (`/Game/Player/Blueprints/NoteSystem/BP_Note.StaticMesh1` _asbp_note) "BlockAll" true)
      (set `self.InitialTransform` (`self.GetTransform`))
      (`/Game/Player/Blueprints/Interact/BP_Inspecting.TransferItem` _returnvalue self Player (`KismetMathLibrary.MakeTransform` (0.0 0.0 0.0) (`self.Inspect Rotation `) (`self.Inspect Scale`)) (`self.ItemName`) (`self.ItemDescription`)))))

(fn `ReturnToInitialPosition`
  (bind _asbp_note (cast `/Game/Player/Blueprints/NoteSystem/BP_Note` (`ChildActorComponent.ChildActor` (`self.ChildActor`))))
  (`PrimitiveComponent.SetCollisionProfileName` (`/Game/Player/Blueprints/NoteSystem/BP_Note.StaticMesh1` _asbp_note) "NoCollision" true)
  (`self.K2_DetachFromActor` "KeepWorld" "KeepWorld" "KeepWorld")
  (`self.K2_SetActorTransform` (`self.InitialTransform`) false true)
  (`PrimitiveComponent.SetSimulatePhysics` (`self.StaticMesh`) true))

(fn `SpawnDuplicate`
  (params (CamRef :type "SceneCaptureComponent2D Object Reference") (DuplicateTransform :type "Transform Structure"))
  (bind _asbp_fp_character (cast `/Game/Player/Blueprints/BP_FP_Character` (`GameplayStatics.GetPlayerCharacter` 0)))
  (bind _camera (`/Game/Player/Blueprints/BP_FP_Character.Camera` _asbp_fp_character))
  (bind _returnvalue (`|SpawnActorFromClass` "BP_InspectableItem_C" (`KismetMathLibrary.MakeTransform` (+ (- (.location (`self.GetTransform`)) (`SceneComponent.K2_GetComponentLocation` CamRef)) (* (`SceneComponent.GetForwardVector` _camera) -402.0) (`SceneComponent.K2_GetComponentLocation` _camera)) (.rotation DuplicateTransform) (.scale DuplicateTransform)) "Undefined" "MultiplyWithRoot" null (`self.HasNote`) (`self.NoteTransform`) true (`self.ItemMesh`) null))
  (bind _output_get (set `self.DuplicateRef` _returnvalue))
  (`PrimitiveComponent.SetSimulatePhysics` (`/Game/Player/Blueprints/Interact/Items/BP_BaseItem.StaticMesh` _output_get) false))

(fn `UpdateDuplicate`
  (`self.K2_SetActorRotation` (`self.DuplicateRef`) (`self.K2_GetActorRotation`) false))

(fn `UserConstructionScript`
  (`parent.UserConstructionScript`)
  (if (`self.HasNote`)
    (`ChildActorComponent.SetChildActorClass` (`self.ChildActor`) "/Game/Player/Blueprints/NoteSystem/BP_Note.BP_Note_C")
    (`SceneComponent.K2_SetRelativeTransform` (`self.ChildActor`) (`self.NoteTransform`) false false)
    (bind _asbp_note (cast `/Game/Player/Blueprints/NoteSystem/BP_Note` (`ChildActorComponent.ChildActor` (`self.ChildActor`))))
    (set `/Game/Player/Blueprints/NoteSystem/BP_Note.NoteLetter` (`self.Note`) _asbp_note)
    (else
      (`ChildActorComponent.SetChildActorClass` (`self.ChildActor`) null)))
  (if (`self.IsDuplicate`)
    (`SceneComponent.SetVisibility` (`self.StaticMesh`) false true)))