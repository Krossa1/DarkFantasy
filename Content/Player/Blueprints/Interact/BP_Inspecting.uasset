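; Temporary actor that runs the item inspection view.
; TransferItem applies the inspect rotation and scale, attaches the item to itself, shows W_Inspect with name and description, and moves input from the player to itself.
; Holding left mouse rotates the item with mouse movement, while right mouse resets the Item component's rotation and the scene capture FOV.
; Interact restores player input, removes the widget, returns the BP_InspectableItem and destroys this actor.
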(event `TransferItem`
  (params (ActorToInspect :type "Actor Object Reference") (PlayerRef :type "/Game/Player/Blueprints/BP_FP_Character Object Reference") (InspectTransform :type "Transform Structure") (ItemName :type Text) (ItemDescription :type Text))
  (bind _returnvalue (`GameplayStatics.GetPlayerController` 0))
  ; Inspect Object
  (set `self.ActorToInspect` ActorToInspect)
  (set `self.Player` PlayerRef)
  (`self.SetInspectRotation` (.rotation InspectTransform))
  (`self.SetInspectScale` (.scale InspectTransform))
  (`self.K2_AttachToActor` (`self.ActorToInspect`) self "None" "SnapToTarget" "KeepRelative" "KeepRelative" true)
  (bind _returnvalue_2 (`|CreateWidget` "/Game/Widgets/W_Inspect.W_Inspect_C" null ItemName ItemDescription))
  (bind _output_get (set `self.InspectWidget` _returnvalue_2))
  (`UserWidget.AddToViewport` _output_get 0)
  (`self.DisableInput` (`self.Player`) _returnvalue)
  (`self.EnableInput` _returnvalue))

(event `EnhancedInput|/Game/Player/InputMappings/Actions/IA_Interact`
  (params (ActionValue :type Boolean) (ElapsedSeconds :type "Float (double-precision)") (TriggeredSeconds :type "Float (double-precision)") (InputAction :type "InputAction Object Reference" :default "/Game/Player/InputMappings/Actions/IA_Interact.IA_Interact"))
  (bind _returnvalue (`GameplayStatics.GetPlayerController` 0))
  (bind _inspectwidget (`self.InspectWidget`))
  ; InteractEvent Handling
  (:`Started`
    (`self.DisableInput` _returnvalue)
    (`self.EnableInput` (`self.Player`) _returnvalue)
    (`/Engine/EditorBlueprintResources/StandardMacros.IsValid` _inspectwidget
      (:`Is Valid`
        (`Widget.RemoveFromParent` _inspectwidget)
        (set `self.InspectWidget` null)
        (bind _asbp_inspectable_item (cast `/Game/Player/Blueprints/Interact/Items/BP_InspectableItem` (`self.ActorToInspect`)))
        (`/Game/Player/Blueprints/Interact/Items/BP_InspectableItem.ReturnToInitialPosition` _asbp_inspectable_item)
        (`self.K2_DestroyActor`)))))

(event `Key|LeftMouseButton`
  (params (Key :type "Key Structure"))
  ; Only Rotate on LMB
  (:`Pressed`
    (set `self.Rotate?` true))
  (:`Released`
    (set `self.Rotate?` false)))

(event `SetInspectRotation`
  (params (`Item Rotation` :type "Rotator Structure"))
  (bind _actortoinspect (`self.ActorToInspect`))
  (bind (_returnvalue_location _returnvalue_rotation _returnvalue_scale) (`KismetMathLibrary.BreakTransform` (`self.GetTransform` _actortoinspect)))
  ; Set Inspect Rotation
  (bind _output_get (set `self.Item Rotation` `Item Rotation`))
  (`self.K2_SetActorTransform` _actortoinspect (`KismetMathLibrary.MakeTransform` _returnvalue_location _output_get _returnvalue_scale) false false))

(event `Key|RightMouseButton`
  (params (Key :type "Key Structure"))
  ; Reset Transform
  (:`Pressed`
    (`SceneComponent.K2_SetWorldRotation` (`self.Item`) (`self.Item Rotation`) false false)
    (set `SceneCaptureComponent2D.FOVAngle` 50.0 (`self.SceneCaptureComponent2D`))))

(event `SetInspectScale`
  (params (`Item Scale` :type "Vector Structure"))
  (bind _actortoinspect (`self.ActorToInspect`))
  (bind (_returnvalue_location _returnvalue_rotation) (`KismetMathLibrary.BreakTransform` (`self.GetTransform` _actortoinspect)))
  ; Set Inspect Scale
  (bind _output_get (set `self.Item Scale` `Item Scale`))
  (`self.K2_SetActorTransform` _actortoinspect (`KismetMathLibrary.MakeTransform` _returnvalue_location _returnvalue_rotation _output_get) false false))

(event `InputAxisKey|MouseX`
  (params (AxisValue :type "Float (single-precision)"))
  ; Set Mouse Movement Horizontally
  (if (`self.Rotate?`)
    (`self.K2_SetActorRotation` (`self.ActorToInspect`) (`KismetMathLibrary.ComposeRotators` (`self.K2_GetActorRotation` (`self.ActorToInspect`)) (`KismetMathLibrary.MakeRotator` 0.0 0.0 (* AxisValue -3.0))) false)))

(event `InputAxisKey|MouseY`
  (params (AxisValue :type "Float (single-precision)"))
  ; Set Mouse Movement Vertically
  (if (`self.Rotate?`)
    (`self.K2_SetActorRotation` (`self.ActorToInspect`) (`KismetMathLibrary.ComposeRotators` (`self.K2_GetActorRotation` (`self.ActorToInspect`)) (`KismetMathLibrary.MakeRotator` 0.0 (* -3.0 AxisValue))) false)))

(fn `UserConstructionScript`)