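; Note-system actor that shows an interaction hint widget when the player character comes within range.
; Entering the inner sphere, sized from InnerSphereRadius at construction, creates a W_Interact for the widget component and plays its ShowInteract animation.
; Leaving reverses the animation, then clears and hides the widget after a short delay, with HintVisible guarding against replays.
; A debug "Hello" print remains on overlap.
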(event `self.InnerSqhereCollision.OnComponentBeginOverlap`
  (params (OverlappedComponent :type "PrimitiveComponent Object Reference") (OtherActor :type "Actor Object Reference") (OtherComp :type "PrimitiveComponent Object Reference") (OtherBodyIndex :type Integer) (bFromSweep :type Boolean) (SweepResult :type "HitResult Structure (by ref)"))
  (bind _widget (`self.Widget`))
  (if (== OtherActor (`GameplayStatics.GetPlayerCharacter` 0))
    (`KismetSystemLibrary.PrintText` "Hello")
    (bind _returnvalue (`|CreateWidget` "/Game/Widgets/W_Interact.W_Interact_C"))
    (bind _output_get (set `self.InteractWidget` _returnvalue))
    (`WidgetComponent.SetWidget` _widget _output_get)
    (`SceneComponent.SetVisibility` _widget true false)
    (bind _interactwidget (`self.InteractWidget`)
      (:`then`
        (`/Game/Widgets/W_Interact.ToggleItem` _interactwidget false)
        (if (not (`self.HintVisible`))
          (`UserWidget.PlayAnimation` _interactwidget (`/Game/Widgets/W_Interact.ShowInteract` _interactwidget) 0.0 1 "Forward" 1.5 false)
          (set `self.HintVisible` true)))
      (:`else`))))

(event `self.InnerSqhereCollision.OnComponentEndOverlap`
  (params (OverlappedComponent :type "PrimitiveComponent Object Reference") (OtherActor :type "Actor Object Reference") (OtherComp :type "PrimitiveComponent Object Reference") (OtherBodyIndex :type Integer))
  (if (== (`GameplayStatics.GetPlayerCharacter` 0) OtherActor)
    (bind _interactwidget (`self.InteractWidget`)
      (:`then`
        (if (`self.HintVisible`)
          (`UserWidget.PlayAnimation` _interactwidget (`/Game/Widgets/W_Interact.ShowInteract` _interactwidget) 0.0 1 "Reverse" 1.5 false)
          (set `self.HintVisible` false))
        (`KismetSystemLibrary.Delay` 0.2)
        (`Widget.RemoveFromParent` (`self.InteractWidget`))
        (set `self.InteractWidget` null)
        (`SceneComponent.SetVisibility` (`self.Widget`) false false))
      (:`else`))))

(fn `UserConstructionScript`
  (`parent.UserConstructionScript`)
  (`SphereComponent.SetSphereRadius` (`self.InnerSqhereCollision`) (`self.Inner Sphere Radius`) true))