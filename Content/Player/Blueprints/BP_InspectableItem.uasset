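; BP_InspectableItem is an interactable item that the player can inspect when its Inspect flag is set.
; On interact, it spawns a BP_Inspecting actor at an extremely distant X coordinate, away from the level.
; It passes that actor its inspect rotation and scale, prints the item name, then calls InspectItem with the player, static mesh, name and description.
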(event `/Game/Player/Blueprints/BPI_InteractInterface.OnInteract`
  (params (Player :type "/Game/Player/Blueprints/BP_FP_Character Object Reference"))
  (bind _itemname (`self.ItemName`))
  ; Inspect Item
  (if (`self.Inspect?`)
    (bind _returnvalue (`|SpawnActorFromClass` "/Game/Player/Blueprints/Inspect/BP_Inspecting.BP_Inspecting_C" (`KismetMathLibrary.MakeTransform` (100000000000000.0 0.0 0.0)) "Undefined" "MultiplyWithRoot" null null))
    (`/Game/Player/Blueprints/Inspect/BP_Inspecting.SetInspectRotation` _returnvalue (`self.Inspect Rotation `))
    (`/Game/Player/Blueprints/Inspect/BP_Inspecting.SetInspectScale` _returnvalue (`self.Inspect Scale`))
    (`KismetSystemLibrary.PrintText` _itemname)
    (`/Game/Player/Blueprints/Inspect/BP_Inspecting.Inspect Item` _returnvalue Player (`StaticMeshComponent.StaticMesh` (`self.StaticMesh`)) _itemname (`self.ItemDescription`))))

(fn `UserConstructionScript`
  (`parent.UserConstructionScript`))