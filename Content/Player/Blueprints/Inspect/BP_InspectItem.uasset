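; Inspection actor that displays a given item's mesh alongside the W_Inspect widget.
; Its Inspect event stores the player, sets the Item mesh, adds the widget to the viewport and toggles input on the first player controller.
; Test code caches BP_FP_Character on BeginPlay and prints a debug string each Tick while that character interacts with this actor.
; The Interact function is a stub returning false.
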(event `/Game/Player/Blueprints/BP_InteractInterface.Inspect`
  (params (Player :type "/Game/Player/Blueprints/BP_FP_Character Object Reference") (InspectedItem :type "StaticMesh Object Reference"))
  (bind _returnvalue (`GameplayStatics.GetPlayerController` 0))
  ; Inspect Object
  (set `self.Player` Player)
  (`StaticMeshComponent.SetStaticMesh` (`self.Item`) InspectedItem)
  (bind _returnvalue_2 (`|CreateWidget` "/Game/Player/Blueprints/Inspect/W_Inspect.W_Inspect_C"))
  (bind _output_get (set `self.InspectWidget` _returnvalue_2))
  (`UserWidget.AddToViewport` _output_get 0)
  (`self.DisableInput` _returnvalue)
  (`self.EnableInput` _returnvalue))

(event `self.ReceiveBeginPlay`
  ; Testing Interact
  (bind _asbp_fp_character (cast `/Game/Player/Blueprints/BP_FP_Character` (`GameplayStatics.GetPlayerCharacter` 0)))
  (set `self.BP Player Ref` _asbp_fp_character))

(event `self.ReceiveTick`
  (params (DeltaSeconds :type "Float (single-precision)"))
  (bind _bp_player_ref (`self.BP Player Ref`))
  ; Testing Interact
  (if (and (`/Game/Player/Blueprints/BP_FP_Character.Is Interacting?` _bp_player_ref) (== (`/Game/Player/Blueprints/BP_FP_Character.Hit Actor` _bp_player_ref) self))
    (`KismetSystemLibrary.PrintString` "hi")))

(fn `Interact`
  (params (Player :type "Character Object Reference"))
  (returns (`Did Interact?` :type Boolean))
  (return false))

(fn `UserConstructionScript`)